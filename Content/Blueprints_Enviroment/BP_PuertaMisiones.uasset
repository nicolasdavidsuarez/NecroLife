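; BP_PuertaMisiones is a quest door that opens and destroys itself when the player has the required quest or the boss dies.
; Overlapping its box as NecroLifeCharacter checks QuestNecesaria on the GameState's QuestComponent.
; The boss's death event also teleports the second BP_NecroLifeNpcBasic found to just above NewLocation.
; Both triggers activate Niagara and run looping timers that slide the door with decelerating offsets until TiempoFadeOut elapses.
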(event OnComponentBeginOverlap(BoxCollision)
  (params (OverlappedComponent :type Primitive%20Component%20Object%20Reference) (OtherActor :type Actor%20Object%20Reference) (OtherComp :type Primitive%20Component%20Object%20Reference) (OtherBodyIndex :type Integer) (bFromSweep :type Boolean) (SweepResult :type Hit%20Result%20Structure%20%28by%20ref%29))
  (Utilities|Casting|CastToNecroLifeCharacter OtherActor)
  (bind _returnvalue (Class|QuestComponent|HasQuest (Actor|GetComponentbyClass (Game|GetGameState) "/Script/NecroLife.QuestComponent") (Variables|Default|GetQuestNecesaria)))
  (if _returnvalue
    (Components|Activation|Activate (Variables|Default|GetNiagara) false)
    (bind _returnvalue_2 (Utilities|Time|SetTimerbyEvent (delegate Custom|fadeOut) 0.01 true true))))

(event Custom|AbrePuerta
  (Transformation|AddActorLocalOffset (Math|Vector|MakeVector 0.0 (* -2.0 (- 1.0 (/ (Variables|Default|GettiempoAcumulado) (Variables|Default|GettiempoFadeOut)))) 0.0) false false)
  (bind _output_get (Variables|Default|SettiempoAcumulado (+ (Variables|Default|GettiempoAcumulado) 0.01)))
  (if (> _output_get (Variables|Default|GettiempoFadeOut))
    (Utilities|Time|ClearandInvalidateTimerbyHandle (stale Custom|CustomEvent _returnvalue))
    (Actor|DestroyActor)))

(event Custom|fadeOut
  (Transformation|AddActorLocalOffset (Math|Vector|MakeVector 0.0 (* -2.0 (- 1.0 (/ (Variables|Default|GettiempoAcumulado) (Variables|Default|GettiempoFadeOut)))) 0.0) false false)
  (bind _output_get (Variables|Default|SettiempoAcumulado (+ (Variables|Default|GettiempoAcumulado) 0.01)))
  (if (> _output_get (Variables|Default|GettiempoFadeOut))
    (Utilities|Time|ClearandInvalidateTimerbyHandle (stale OnComponentBeginOverlap(BoxCollision) _returnvalue_2))
    (Actor|DestroyActor)))

(event Custom|CustomEvent
  (params (Enemy :type Necro%20Life%20Enemy%20Basic%20Object%20Reference))
  (bind _new_location (Variables|Default|GetNew%20Location))
  (bind _outactors (Actor|GetAllActorsOfClass "/Game/Characters/Npc/BP_NecroLifeNpcBasic.BP_NecroLifeNpcBasic_C"))
  (Transformation|SetActorLocation (Utilities|Array|Get(acopy) _outactors 1) (Math|Vector|MakeVector (.x _new_location) (.y _new_location) (+ (.z _new_location) 1e+02)) false false)
  (Components|Activation|Activate (Variables|Default|GetNiagara) false)
  (bind _returnvalue (Utilities|Time|SetTimerbyEvent (delegate Custom|AbrePuerta) 0.01 true true)))

(event EventBeginPlay
  (bind _returnvalue (Actor|GetActorOfClass "/Game/Maps/PlayGround/Blueprints/BP_EnemyBoss.BP_EnemyBoss_C"))
  (bind _output_get (Variables|Default|SetBoss _returnvalue))
  (EventDispatchers|BindEventtoOnEnemyDied _output_get (delegate Custom|CustomEvent)))

(event Collision|EventActorBeginOverlap
  (params (OtherActor :type Actor%20Object%20Reference)))

(event EventTick
  (params (DeltaSeconds :type Float%20%28single-precision%29)))

(fn ConstructionScript)