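; Village fountain that gives BP_Huesos water for the forest fire quest when the character walks into its collision sphere.
; Overlap registers the fountain as the current interactable, and leaving clears it.
; If the GameState QuestComponent has the quest and the character never had a barrel, it advances the fountain objective.
; It then adds water to the PlayerState inventory, shows the barrel, sets its flags and activates Niagara.
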(event OnComponentBeginOverlap(SphereCollision)
  (params (OverlappedComponent :type Primitive%20Component%20Object%20Reference) (OtherActor :type Actor%20Object%20Reference) (OtherComp :type Primitive%20Component%20Object%20Reference) (OtherBodyIndex :type Integer) (bFromSweep :type Boolean) (SweepResult :type Hit%20Result%20Structure%20%28by%20ref%29))
  (bind _returnvalue (Game|GetGameState))
  (bind _returnvalue_2 (Actor|GetComponentbyClass _returnvalue "/Script/NecroLife.QuestComponent"))
  (bind _asbp_huesos (Utilities|Casting|CastToBP_Huesos OtherActor))
  (Class|NecroLifeCharacter|SetCurrentInteractable _asbp_huesos self)
  (if (not (Variables|/Game/Characters/Playable_Characters/BP_Huesos.BP_Huesos_C|GetbTuvoBarril _asbp_huesos))
    (bind _returnvalue_3 (Class|QuestComponent|HasQuest _returnvalue_2 "/Game/Maps/PlayGround/Data_Assets/DA_QuestFuegoBosque.DA_QuestFuegoBosque"))
    (if _returnvalue_3
      (Class|QuestComponent|UpdateQuestProgress _returnvalue_2 "(TagName=\"Necro_Tags.MisionFuegoBosque.FuentePueblo\")" 1)
      (if (Utilities|IsValid _returnvalue_2)
        (Class|InventoryComponent|PickUp (Actor|GetComponentbyClass (Variables|/Script/Engine.Pawn|GetPlayerState _asbp_huesos) "/Script/NecroLife.InventoryComponent") "/Game/Assets/DataAssets/ID_Agua_Fuente.ID_Agua_Fuente")
        (Default|MostrarBarril _asbp_huesos)
        (Variables|/Game/Characters/Playable_Characters/BP_Huesos.BP_Huesos_C|SetbTieneBarril _asbp_huesos true)
        (Variables|/Game/Characters/Playable_Characters/BP_Huesos.BP_Huesos_C|SetbTuvoBarril _asbp_huesos true)
        (Components|Activation|Activate (Variables|/Game/Characters/Playable_Characters/BP_Huesos.BP_Huesos_C|GetNiagara _asbp_huesos) false)))))

(event OnComponentEndOverlap(SphereCollision)
  (params (OverlappedComponent :type Primitive%20Component%20Object%20Reference) (OtherActor :type Actor%20Object%20Reference) (OtherComp :type Primitive%20Component%20Object%20Reference) (OtherBodyIndex :type Integer))
  (bind _asbp_huesos (Utilities|Casting|CastToBP_Huesos OtherActor))
  (Class|NecroLifeCharacter|ClearCurrentInteractable _asbp_huesos))

(event EventBeginPlay)

(event EventTick
  (params (DeltaSeconds :type Float%20%28single-precision%29)))

(fn ConstructionScript)