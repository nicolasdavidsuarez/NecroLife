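; BP_LlegarLugar is a trigger volume that advances a quest objective when BP_Huesos reaches its location.
; On BeginPlay it sizes its Box from the extent variables.
; Box overlaps with a BP_Huesos call UpdateQuestProgress on the GameState's QuestComponent with the objective ID and amount.
; It has no one-shot guard, so each new overlap reports progress again.
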(event OnComponentBeginOverlap(Box)
  (params (OverlappedComponent :type Primitive%20Component%20Object%20Reference) (OtherActor :type Actor%20Object%20Reference) (OtherComp :type Primitive%20Component%20Object%20Reference) (OtherBodyIndex :type Integer) (bFromSweep :type Boolean) (SweepResult :type Hit%20Result%20Structure%20%28by%20ref%29))
  (Utilities|Casting|CastToBP_Huesos OtherActor)
  (Class|QuestComponent|UpdateQuestProgress (Actor|GetComponentbyClass (Game|GetGameState) "/Script/NecroLife.QuestComponent") (Variables|Default|GetObjective%20ID) (Variables|Default|GetAmount)))

(event EventBeginPlay
  (Components|Box|SetBoxExtent (Variables|Default|GetBox) (Math|Vector|MakeVector (Variables|Default|GetIn%20Box%20Extent%20X) (Variables|Default|GetIn%20Box%20Extent%20Y) 0.0) true))

(event Collision|EventActorBeginOverlap
  (params (OtherActor :type Actor%20Object%20Reference)))

(event EventTick
  (params (DeltaSeconds :type Float%20%28single-precision%29)))

(fn ConstructionScript)