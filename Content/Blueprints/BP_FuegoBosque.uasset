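; Interactable forest fire that BP_Huesos characters put out with fountain water as a quest objective.
; Overlapping CollisionFire registers it as the character's current interactable, and interacting routes the request through the character's ServerApagarFuego.
; Server_ApagarFuego searches the player's PlayerState inventory for water, then removes it and advances the MisionFuegoBosque objective on the GameState QuestComponent.
; A multicast deactivates the Niagara fire and has the character remove its barrel.
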(event OnComponentBeginOverlap(CollisionFire)
  (params (OverlappedComponent :type Primitive%20Component%20Object%20Reference) (OtherActor :type Actor%20Object%20Reference) (OtherComp :type Primitive%20Component%20Object%20Reference) (OtherBodyIndex :type Integer) (bFromSweep :type Boolean) (SweepResult :type Hit%20Result%20Structure%20%28by%20ref%29))
  (bind _asbp_huesos (Utilities|Casting|CastToBP_Huesos OtherActor))
  (Class|NecroLifeCharacter|SetCurrentInteractable _asbp_huesos self))

(event OnComponentEndOverlap(CollisionFire)
  (params (OverlappedComponent :type Primitive%20Component%20Object%20Reference) (OtherActor :type Actor%20Object%20Reference) (OtherComp :type Primitive%20Component%20Object%20Reference) (OtherBodyIndex :type Integer))
  (bind _asbp_huesos (Utilities|Casting|CastToBP_Huesos OtherActor))
  (Class|NecroLifeCharacter|ClearCurrentInteractable _asbp_huesos))

(event Custom|Server_ApagarFuego
  (params (Interactor :type Actor%20Object%20Reference))
  (bind _asbp_huesos (Utilities|Casting|CastToBP_Huesos Interactor))
  (bind _returnvalue (Class|InventoryComponent|GetItemsinInventory (Actor|GetComponentbyClass (Variables|/Script/Engine.Pawn|GetPlayerState _asbp_huesos) "/Script/NecroLife.InventoryComponent")))
  (for _array_element _returnvalue
    (if (== _array_element "/Game/Assets/DataAssets/ID_Agua_Fuente.ID_Agua_Fuente")
      (Development|PrintString "tiene agua!!!!!!!!!!!!!!!!" true true "(R=0.000000,G=0.660000,B=1.000000,A=1.000000)" 6.0)
      (Utilities|Array|RemoveItem _returnvalue "/Game/Assets/DataAssets/ID_Agua_Fuente.ID_Agua_Fuente")
      (Components|Activation|Deactivate (Variables|Default|GetNiagara))
      (Class|QuestComponent|UpdateQuestProgress (Actor|GetComponentbyClass (Game|GetGameState) "/Script/NecroLife.QuestComponent") "(TagName=\"Necro_Tags.MisionFuegoBosque.FuegoBosque\")" 1)
      (CallFunction|MulticastApagarFuego Interactor)
      (else
        (Development|PrintString "no pasa el branch del fuego")))))

(event Custom|Multicast_ApagarFuego
  (params (Interactor :type Actor%20Object%20Reference))
  (Components|Activation|Deactivate (Variables|Default|GetNiagara))
  (bind _asbp_huesos (Utilities|Casting|CastToBP_Huesos Interactor))
  (Default|MulticastQuitarBarril _asbp_huesos))

(event EventBeginPlay
  (Class|NiagaraComponent|SetAsset (Variables|Default|GetNiagara) "/Game/FX/NS_FuegoBosque.NS_FuegoBosque" true))

(event Collision|EventActorBeginOverlap
  (params (OtherActor :type Actor%20Object%20Reference)))

(event EventTick
  (params (DeltaSeconds :type Float%20%28single-precision%29)))

(event EventOnInteract
  (params (Interactor :type Actor%20Object%20Reference))
  (bind _asbp_huesos (Utilities|Casting|CastToBP_Huesos Interactor))
  (Default|ServerApagarFuego _asbp_huesos self))

(fn ConstructionScript)