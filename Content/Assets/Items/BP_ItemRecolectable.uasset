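; BP_ItemRecolectable is a collectible item that advances a quest objective when a NecroLifeCharacter overlaps its sphere.
; BeginPlay applies the Mesh variable to ItemMesh.
; On overlap, it finds the QuestComponent on the GameState, adds one progress to ObjectiveIDTag and prints the component's name as debug text.
; The item neither destroys nor disables itself, so each new overlap counts again.
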(event OnComponentBeginOverlap(SphereCollision)
  (params (OverlappedComponent :type Primitive%20Component%20Object%20Reference) (OtherActor :type Actor%20Object%20Reference) (OtherComp :type Primitive%20Component%20Object%20Reference) (OtherBodyIndex :type Integer) (bFromSweep :type Boolean) (SweepResult :type Hit%20Result%20Structure%20%28by%20ref%29))
  (bind _returnvalue (Game|GetGameState))
  (bind _returnvalue_2 (Actor|GetComponentbyClass _returnvalue "/Script/NecroLife.QuestComponent"))
  (Utilities|Casting|CastToNecroLifeCharacter OtherActor)
  (if (Utilities|IsValid _returnvalue_2)
    (Class|QuestComponent|UpdateQuestProgress _returnvalue_2 (Variables|Default|GetObjective%20ID%20Tag) 1)
    (Development|PrintString (Utilities|GetDisplayName _returnvalue_2) true true "(R=1.000000,G=0.974254,B=0.000000,A=1.000000)" 5.0)))

(event EventBeginPlay
  (Components|StaticMesh|SetStaticMesh (Variables|Default|GetItemMesh) (Variables|Default|GetMesh)))

(event EventTick
  (params (DeltaSeconds :type Float%20%28single-precision%29)))

(fn ConstructionScript)