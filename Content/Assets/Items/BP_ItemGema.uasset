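; Gem item actor whose look reflects the attribute it improves.
; The construction script reads its GemaId data table row and switches on AtributoAMejorar to set the mesh and material, with several attributes sharing looks.
; Defense gems use the HPRegen mesh, while life regeneration gems use the Defense mesh with the HP material.
; At play, a looping timer rotates the actor in fixed steps instead of using Tick.
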(event Custom|Movimiento
  (Transformation|AddActorLocalRotation "0.000000,20.000000,0.000000" false false))

(event EventBeginPlay
  (Utilities|Time|SetTimerbyEvent (delegate Custom|Movimiento) 0.09 true))

(event Collision|EventActorBeginOverlap
  (params (OtherActor :type Actor%20Object%20Reference)))

(event EventTick
  (params (DeltaSeconds :type Float%20%28single-precision%29)))

(fn ConstructionScript
  (bind _gema_id (Variables|ItemGema|GetGema_Id))
  (bind _itemmesh (Variables|Default|GetItemMesh))
  (bind _itemmesh_2 (Variables|Default|GetItemMesh))
  (bind _itemmesh_3 (Variables|Default|GetItemMesh))
  (bind _itemmesh_4 (Variables|Default|GetItemMesh))
  (bind _itemmesh_5 (Variables|Default|GetItemMesh))
  (bind _itemmesh_6 (Variables|Default|GetItemMesh))
  (bind _itemmesh_7 (Variables|Default|GetItemMesh))
  (bind (_datatable _rowname) (Utilities|Struct|BreakDataTableRowHandle _gema_id))
  (bind _returnvalue (Utilities|GetDataTableRow _datatable _rowname)
    (:then
      (bind _output_get (Variables|Default|SetGemaData _returnvalue))
      (switch Utilities|FlowControl|Switch|SwitchonETipoEstadisticaGema (.atributoamejorar _output_get)
        (:VidaMaxima
          (Components|StaticMesh|SetStaticMesh _itemmesh_3 "/Game/Arte/SM_Items/SM_Gem_HP.SM_Gem_HP" :!label _label)
          (Rendering|Material|SetMaterial _itemmesh_3 0 "/Game/Arte/Materials/Gems/M_Gem_HP.M_Gem_HP"))
        (:AtaqueFisico
          (Components|StaticMesh|SetStaticMesh _itemmesh_4 "/Game/Arte/SM_Items/SM_Gem_Attack.SM_Gem_Attack" :!label _label_2)
          (Rendering|Material|SetMaterial _itemmesh_4 0 "/Game/Arte/Materials/Gems/M_Gem_Attack.M_Gem_Attack"))
        (:Defensa
          (Components|StaticMesh|SetStaticMesh _itemmesh_5 "/Game/Arte/SM_Items/SM_Gem_HPRegen.SM_Gem_HPRegen" :!label _label_3)
          (Rendering|Material|SetMaterial _itemmesh_5 0 "/Game/Arte/Materials/Gems/M_Gem_Defense.M_Gem_Defense"))
        (:EnergiaMaxima
          (Components|StaticMesh|SetStaticMesh _itemmesh_6 "/Game/Arte/SM_Items/SM_Gem_Energy.SM_Gem_Energy" :!label _label_4)
          (Rendering|Material|SetMaterial _itemmesh_6 0 "/Game/Arte/Materials/Gems/M_Gem_Energy.M_Gem_Energy"))
        (:AtaqueFisicoPorcentaje
          (goto _label_2))
        (:DefensaPorcentaje
          (goto _label_3))
        (:VidaMaximaPorcentaje
          (goto _label))
        (:Velocidad
          (Components|StaticMesh|SetStaticMesh _itemmesh_7 "/Game/Arte/SM_Items/SM_Gem_Velocity.SM_Gem_Velocity")
          (Rendering|Material|SetMaterial _itemmesh_7 0 "/Game/Arte/Materials/Gems/M_Gem_Velocity.M_Gem_Velocity"))
        (:RegeneracionVida
          (Components|StaticMesh|SetStaticMesh _itemmesh "/Game/Arte/SM_Items/SM_Gem_Defense.SM_Gem_Defense")
          (Rendering|Material|SetMaterial _itemmesh 0 "/Game/Arte/Materials/Gems/M_Gem_HP.M_Gem_HP"))
        (:RegeneracionEnergia
          (goto _label_4))
        (:VelocidadAtaquePorcentaje
          (Components|StaticMesh|SetStaticMesh _itemmesh_2 "/Game/Arte/SM_Items/SM_Gem_Velocity.SM_Gem_Velocity")
          (Rendering|Material|SetMaterial _itemmesh_2 0 "/Game/Arte/Materials/Gems/M_Gem_Velocity.M_Gem_Velocity"))))))