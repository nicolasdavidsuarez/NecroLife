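; Ranged enemy character Blueprint that handles health feedback and death; no attack logic appears in its graphs.
; On BeginPlay it binds to the HealthComponent's health-change event and sets a gameplay tag if that tag is valid.
; Health changes update the life bar in its WB_Enemy widget as a fraction of max health.
; At zero health it spawns an XP pickup at its transform and destroys itself.
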(event Custom|muere?
  (params (NewHealth :type Float%20%28single-precision%29) (MaxHealth :type Float%20%28single-precision%29))
  (if (<= NewHealth 0.0)
    (Game|SpawnActorfromClass "/Game/Assets/Items/BP_ItemXP.BP_ItemXP_C" (Transformation|GetActorTransform) "Undefined" "MultiplyWithRoot" 0 0)
    (Actor|DestroyActor)
    (else
      (bind _aswb_enemy (Utilities|Casting|CastToWB_Enemy (UserInterface|GetWidget (Variables|Default|GetWidget))))
      (Default|UpdateLife _aswb_enemy (/ NewHealth MaxHealth)))))

(event EventBeginPlay
  (EventDispatchers|BindEventtoOnHealthChanged (Variables|Default|GetHealthComponent) (delegate Custom|muere?))
  (if (GameplayTags|IsGameplayTagValid)
    (Class|NecroLifeEnemyBasic|SetTag)))

(event Collision|EventActorBeginOverlap
  (params (OtherActor :type Actor%20Object%20Reference)))

(event EventTick
  (params (DeltaSeconds :type Float%20%28single-precision%29)))

(fn ConstructionScript)