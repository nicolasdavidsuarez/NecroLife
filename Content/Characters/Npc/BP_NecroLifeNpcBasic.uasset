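; BP_NecroLifeNpcBasic is a basic NPC that offers itself for interaction when BP_Huesos comes near.
; On sphere overlap by any actor with authority it shows a text prompt, then, for BP_Huesos only, registers as the current interactable and snaps to face it.
; When BP_Huesos leaves the sphere, it clears that interactable and hides the text, without an authority check.
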(event OnComponentBeginOverlap(SphereCollision)
  (params (OverlappedComponent :type Primitive%20Component%20Object%20Reference) (OtherActor :type Actor%20Object%20Reference) (OtherComp :type Primitive%20Component%20Object%20Reference) (OtherBodyIndex :type Integer) (bFromSweep :type Boolean) (SweepResult :type Hit%20Result%20Structure%20%28by%20ref%29))
  (bind _self self)
  (if (Ability|HasAuthority OtherActor)
    (Rendering|SetVisibility (Variables|Default|GetTextRender) true false)
    (bind _asbp_huesos (Utilities|Casting|CastToBP_Huesos OtherActor))
    (Class|NecroLifeCharacter|SetCurrentInteractable _asbp_huesos _self)
    (Transformation|SetActorRotation (Math|Rotator|FindLookatRotation (Transformation|GetActorLocation _self) (Transformation|GetActorLocation OtherActor)))))

(event OnComponentEndOverlap(SphereCollision)
  (params (OverlappedComponent :type Primitive%20Component%20Object%20Reference) (OtherActor :type Actor%20Object%20Reference) (OtherComp :type Primitive%20Component%20Object%20Reference) (OtherBodyIndex :type Integer))
  (bind _asbp_huesos (Utilities|Casting|CastToBP_Huesos OtherActor))
  (Class|NecroLifeCharacter|ClearCurrentInteractable _asbp_huesos)
  (Rendering|SetVisibility (Variables|Default|GetTextRender) false false))

(fn ConstructionScript)