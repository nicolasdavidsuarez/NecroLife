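; BP_Huesos is the playable character Huesos, with shovel melee, target lock-on and a water barrel carried overhead to extinguish forest fires.
; The local player creates the HUD, fills ability slots and recalculates stats from socketed gems.
; Tick feeds position to the minimap and an occlusion-mask material parameter collection.
; Death heals the character and uses a looping timer to raise it from below its last spawn point with collision off.
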(event OnComponentBeginOverlap(PalaHitbox)
  (params (OverlappedComponent :type Primitive%20Component%20Object%20Reference) (OtherActor :type Actor%20Object%20Reference) (OtherComp :type Primitive%20Component%20Object%20Reference) (OtherBodyIndex :type Integer) (bFromSweep :type Boolean) (SweepResult :type Hit%20Result%20Structure%20%28by%20ref%29))
  ;[0.15 0.15 0.15 0.5 36] Ataques Combo básico
  (Class|NecroLifeCharacter|ApplyWeaponHit OtherActor))

(event Custom|Multicast_QuitarBarril
  ;[0.15 0.15 0.15 0.5 32] INTERACCIÓN - Barril agua
  (Variables|Default|SetbTieneBarril false))

(event Custom|Server_ApagarFuego
  (params (BP_FuegoBosque :type BP%20Fuego%20Bosque%20Object%20Reference))
  ;[0.15 0.15 0.15 0.5 32] INTERACCIÓN - Barril agua
  (Default|ServerApagarFuego BP_FuegoBosque self)
  (CallFunction|MulticastQuitarBarril))

(event Custom|ActivarPala
  (bind _palahitbox (Variables|Default|GetPalaHitbox))
  ;[0.15 0.15 0.15 0.5 36] Ataques Combo básico
  (Class|NecroLifeCharacter|ClearWeaponHitMemory)
  (Collision|SetCollisionEnabled _palahitbox "QueryOnly")
  (Rendering|ToggleVisibility _palahitbox false)
  (Development|PrintString "ACTIVADA" true true "(R=1.000000,G=0.701200,B=0.000000,A=1.000000)"))

(event Custom|DesactivarPala
  (bind _palahitbox (Variables|Default|GetPalaHitbox))
  ;[0.15 0.15 0.15 0.5 36] Ataques Combo básico
  (Collision|SetCollisionEnabled _palahitbox "NoCollision")
  (Rendering|ToggleVisibility _palahitbox false)
  (Development|PrintString "ACTIVADA" true true "(R=1.000000,G=0.128498,B=0.000000,A=1.000000)"))

(event Custom|reSpawn
  (bind _lastlocationspawn (Variables|Default|GetLastLocationSpawn))
  ;[0.15 0.15 0.15 0.5 36] Muerte - Respawn
  (Transformation|SetActorLocation (Math|Vector|MakeVector (.x _lastlocationspawn) (.y _lastlocationspawn) (- (.z _lastlocationspawn) (Variables|Default|GetSpawnLocationShift))) false false)
  (bind _output_get (Variables|Default|SetSpawnLocationShift (Utilities|Operators|Subtract (Variables|Default|GetSpawnLocationShift) (* (stale EventTick DeltaSeconds) 8e+01))))
  (Development|PrintString (Utilities|String|ToString(Float) _output_get))
  (if (<= _output_get 0.0)
    (Utilities|Time|ClearandInvalidateTimerbyHandle (stale EventOnDie _returnvalue))
    (Variables|Default|SetSpawnLocationShift 3e+02)
    (Collision|SetCollisionEnabled (Variables|Character|GetMesh) "QueryAndPhysics")))

(event Input|EnhancedActionEvents|EnhancedInputActionIA_LockOn
  (params (ActionValue :type Boolean) (ElapsedSeconds :type Float%20%28double-precision%29) (TriggeredSeconds :type Float%20%28double-precision%29) (InputAction :type Input%20Action%20Object%20Reference :default "/Game/Input/Actions/IA_LockOn.IA_LockOn"))
  ;[0.1337 0.15 0.09367 0.5 32] Sistema de Targeting (Lock-on)
  (:Started
    (Class|NecroLifeCharacter|ToggleTargeting)))

(event Input|EnhancedActionEvents|EnhancedInputActionIA_TargetLeft
  (params (ActionValue :type Boolean) (ElapsedSeconds :type Float%20%28double-precision%29) (TriggeredSeconds :type Float%20%28double-precision%29) (InputAction :type Input%20Action%20Object%20Reference :default "/Game/Input/Actions/IA_TargetLeft.IA_TargetLeft"))
  ;[0.1337 0.15 0.09367 0.5 32] Sistema de Targeting (Lock-on)
  (:Started
    (Class|NecroLifeCharacter|SwitchTargetLeft)))

(event Input|EnhancedActionEvents|EnhancedInputActionIA_TargetRight
  (params (ActionValue :type Boolean) (ElapsedSeconds :type Float%20%28double-precision%29) (TriggeredSeconds :type Float%20%28double-precision%29) (InputAction :type Input%20Action%20Object%20Reference :default "/Game/Input/Actions/IA_TargetRight.IA_TargetRight"))
  ;[0.1337 0.15 0.09367 0.5 32] Sistema de Targeting (Lock-on)
  (:Started
    (Class|NecroLifeCharacter|SwitchTargetRight)))

(event EventBeginPlay
  (bind _palahitbox (Variables|Default|GetPalaHitbox))
  (if (Pawn|IsLocallyControlled)
    (bind _returnvalue (UserInterface|CreateWidget "/Game/Widget/UX_UI/WB_Hud.WB_Hud_C" 0 self))
    (Variables|Default|SetHubWidget _returnvalue)
    (bind _output_get (Variables|Default|Setref%20Hub _returnvalue))
    (CallFunction|SetAbilitySlots)
    (UserInterface|Viewport|AddtoViewport _output_get 0)
    (bind _aswb_nombre_player (Utilities|Casting|CastToWB_NombrePlayer (UserInterface|GetUserWidgetObject (Variables|Default|GetWidget))))
    (Default|SetName _aswb_nombre_player (Utilities|String|StringToName (Utilities|GetDisplayName (Class|WidgetComponent|GetOwnerPlayer (Variables|Default|GetWidget)))))
    (Variables|Default|SetWeaponMesh 0)
    (bind _asnecro_life_player_state (Utilities|Casting|CastToNecroLifePlayerState (Variables|/Script/Engine.Controller|GetPlayerState (Pawn|GetController))))
    (Class|AttributeComponent|RecalcularEstadisticas (Variables|/Script/NecroLife.NecroLifePlayerState|GetAttributeComponent _asnecro_life_player_state) (Variables|/Script/NecroLife.InventoryComponent|GetGemsInSlots (Variables|Default|GetInventory)))
    (Collision|SetCollisionEnabled _palahitbox "NoCollision")
    (Rendering|ToggleVisibility _palahitbox false)))

(event EventBpSpawnReward
  ;[0.15 0.15 0.15 0.5] Rewards
  (Game|SpawnActorfromClass "/Game/Assets/Items/BP_ItemGema.BP_ItemGema_C" (Transformation|GetActorTransform) "Undefined" "MultiplyWithRoot" 0 (Utilities|Array|Get(acopy) (Variables|Default|GetGema%20Id) (Variables|Default|GetposGema)) 0)
  (Variables|Default|SetposGema (+ (Variables|Default|GetposGema) 1)))

(event EventTick
  (params (DeltaSeconds :type Float%20%28single-precision%29))
  (bind _returnvalue (Math|Random|RandomFloatinRange 0.98 1.0))
  (bind _returnvalue_2 (Transformation|GetActorLocation))
  (bind _staticmeshcabeza (Variables|Default|GetStaticMeshCabeza))
  (bind _ref_hub (Variables|Default|Getref%20Hub))
  (Rendering|Material|SetVectorParameterValue "/Game/Maps/PlayGround/Materials/MPC_OclusionMask.MPC_OclusionMask" "PlayerPosicion" (Utilities|Struct|MakeLinearColor (.x _returnvalue_2) (.y _returnvalue_2) (.z _returnvalue_2) (Variables|/Script/Engine.SpringArmComponent|GetTargetArmLength (Variables|Default|GetCameraBoom))) :!class /Script/Engine.KismetMaterialLibrary)
  (if (Utilities|IsValid _ref_hub)
    (bind _aswb_hud (Utilities|Casting|CastToWB_Hud _ref_hub))
    (Default|ActualizarMiniMapa _aswb_hud (.x _returnvalue_2) (.y _returnvalue_2) (Math|Rotator|MakeRotator 0.0 0.0 (.yaw (Transformation|GetActorRotation))))
    (if (Variables|Default|GetbTieneBarril)
      (Transformation|ResetRelativeTransform _staticmeshcabeza)
      (Transformation|AddLocalOffset _staticmeshcabeza (Math|Vector|MakeVector 0.0 0.0 (* _returnvalue 2.7e+02)) false false)
      (Transformation|AddLocalRotation _staticmeshcabeza (Math|Rotator|MakeRotator _returnvalue _returnvalue 0.0) false false))))

(event EventSetCoolDownAbility
  (params (slot :type Integer))
  (bind _aswb_hud (Utilities|Casting|CastToWB_Hud (Variables|Default|Getref%20Hub)))
  (Default|CoolDownAbility _aswb_hud slot))

(event EventOnDie
  (bind _lastlocationspawn (Variables|Default|GetLastLocationSpawn))
  (bind _healthcomponent (Variables|Default|GetHealthComponent))
  ;[0.15 0.15 0.15 0.5 36] Muerte - Respawn
  (Utilities|FlowControl|Delay 3.0)
  (Collision|SetCollisionEnabled (Variables|Character|GetMesh) "NoCollision")
  (Class|UHealthComponent|ApplyHealing _healthcomponent (Variables|/Script/NecroLife.UHealthComponent|GetMaxHealth _healthcomponent))
  (Transformation|SetActorLocation (Math|Vector|MakeVector (.x _lastlocationspawn) (.y _lastlocationspawn) (- (.z _lastlocationspawn) (Variables|Default|GetSpawnLocationShift))) false false)
  (Components|Activation|Activate (Variables|Default|GetNiagaraSpawn) false)
  (bind _returnvalue (Utilities|Time|SetTimerbyEvent (delegate Custom|reSpawn) (stale EventTick DeltaSeconds) true)))

(event Input|KeyboardEvents|Escape
  (params (Key :type Key%20Structure :default "None"))
  ;[0.15 0.15 0.15 0.5 32] MENÚ PAUSA
  (:Pressed
    (bind _aswb_hud (Utilities|Casting|CastToWB_Hud (Variables|Default|Getref%20Hub)))
    (Default|MostrarPausa _aswb_hud)))

(fn ConstructionScript)

(fn GetLookatLocation
  (return "0, 0, 0"))

(fn SetAbilitySlots
  (bind _aswb_hud (Utilities|Casting|CastToWB_Hud (Variables|Default|Getref%20Hub)))
  (bind _returnvalue (Class|AbilityComponent|GetAbilitySlots (Variables|Default|GetAbility)))
  (Default|SetAbilitiesSlots (Variables|/Game/Widget/UX_UI/WB_Hud.WB_Hud_C|GetWB_AbilityPanel _aswb_hud) _returnvalue))

(fn ActualizarForgeInventory
  (bind _aswb_hud (Utilities|Casting|CastToWB_Hud (Variables|Default|Getref%20Hub)))
  (bind _returnvalue (Class|InventoryComponent|GetGemsItemsinInventory (Variables|Default|GetInventory)))
  (Default|LoadGems (Variables|/Game/Widget/UX_UI/WB_Hud.WB_Hud_C|GetWB_InventarioForga _aswb_hud) _returnvalue))

(fn OnRepBTieneBarril
  (bind _staticmeshcabeza (Variables|Default|GetStaticMeshCabeza))
  (if (Variables|Default|GetbTieneBarril)
    (Rendering|SetVisibility _staticmeshcabeza true true)
    (Components|Activation|Activate (Variables|Default|GetNiagara) false)
    (else
      (Rendering|SetVisibility _staticmeshcabeza false true)
      (Components|Activation|Deactivate (Variables|Default|GetNiagara)))))

(fn MostrarBarril
  (bind _staticmeshcabeza (Variables|Default|GetStaticMeshCabeza))
  (Components|StaticMesh|SetStaticMesh _staticmeshcabeza "/Game/Arte/SM_PuebloUmba/SM_SM_Barril_01.SM_SM_Barril_01")
  (Rendering|SetVisibility _staticmeshcabeza true true)
  (Components|Activation|Activate (Variables|Default|GetNiagara) false)
  (Variables|Default|SetbTieneBarril true))