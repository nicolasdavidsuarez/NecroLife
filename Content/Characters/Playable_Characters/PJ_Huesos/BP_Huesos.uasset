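; Blueprint for Huesos, a playable NecroLife character, which connects the character's components to its HUD and handles lock-on targeting input.
; When locally controlled, BeginPlay creates WB_Hub and binds health, XP, inventory, potion, quest, gem and ability cooldown events to it.
; Tick writes player position and camera boom length to an occlusion-mask material parameter collection and updates the minimap.
; OnInteract is empty, with its NPC-to-HUD logic left disconnected.
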(event Custom|ActualizarPotions
  (params (CantPosiones :type Integer))
  (Variables|/Script/UMG.TextBlock|SetText (Variables|/Game/Widget/UX_UI/WB_Hub.WB_Hub_C|Gettxt_posiones (Variables|Default|Getref%20Hub)) (Utilities|Text|ToText(String) (Utilities|String|Append "Posions: " (Utilities|String|ToString(Integer) CantPosiones)))))

(event Custom|actualizarHub
  (params (NewHealth :type Float%20%28single-precision%29) (MaxHealth :type Float%20%28single-precision%29))
  (Default|UpdateLifeBar (Variables|Default|Getref%20Hub) (/ NewHealth MaxHealth)))

(event Custom|ActualizarXpBar
  (params (XP :type Float%20%28single-precision%29) (XPtoNextLevel :type Float%20%28single-precision%29))
  (Default|UpdateXPBar (Variables|Default|Getref%20Hub) (/ XP XPtoNextLevel) (Utilities|String|Append "Nivel: " (Utilities|String|ToString(Integer) (Variables|/Script/NecroLife.AttributeComponent|GetLevel (Variables|Default|GetAttribute))))))

(event Custom|ActualizarInventario
  (params (ItemsToShow :type Array%20of%20Item%20Data%20Object%20References))
  (Default|UpdateInventory (Variables|Default|Getref%20Hub) ItemsToShow))

(event Custom|ActualizarListaObjetivos
  (params (ItemsToMisionList :type Array%20of%20Quest%20UI%20Data%20Structures))
  (Default|ActualizarListaDeMisiones (Variables|Default|Getref%20Hub) ItemsToMisionList))

(event Custom|abilityCoolDown
  (params (AbilitySlot :type Integer))
  (Default|CoolDownAbility (Variables|Default|Getref%20Hub) AbilitySlot))

(event Custom|gemsToShow
  (params (GemsToShow :type Array%20of%20Datos%20Gema%20Structures))
  (Default|SetGemstoGrid (Variables|Default|Getref%20Hub) GemsToShow))

(event Input|EnhancedActionEvents|EnhancedInputActionIA_LockOn
  (params (ActionValue :type Boolean) (ElapsedSeconds :type Float%20%28double-precision%29) (TriggeredSeconds :type Float%20%28double-precision%29) (InputAction :type Input%20Action%20Object%20Reference :default "/Game/Input/Actions/IA_LockOn.IA_LockOn"))
  ;[0.1337 0.15 0.09367 0.5 32] Sistema de Targeting (Lock-on)
  (:Started
    (Class|NecroLifeCharacter|ToggleTargeting)))

(event Input|EnhancedActionEvents|EnhancedInputActionIA_TargetLeft
  (params (ActionValue :type Boolean) (ElapsedSeconds :type Float%20%28double-precision%29) (TriggeredSeconds :type Float%20%28double-precision%29) (InputAction :type Input%20Action%20Object%20Reference :default "/Game/Input/Actions/IA_TargetLeft.IA_TargetLeft"))
  ;[0.1337 0.15 0.09367 0.5 32] Sistema de Targeting (Lock-on)
  (:Started
    (Class|NecroLifeCharacter|SwitchTargetLeft)))

(event Input|EnhancedActionEvents|EnhancedInputActionIA_TargetRight
  (params (ActionValue :type Boolean) (ElapsedSeconds :type Float%20%28double-precision%29) (TriggeredSeconds :type Float%20%28double-precision%29) (InputAction :type Input%20Action%20Object%20Reference :default "/Game/Input/Actions/IA_TargetRight.IA_TargetRight"))
  ;[0.1337 0.15 0.09367 0.5 32] Sistema de Targeting (Lock-on)
  (:Started
    (Class|NecroLifeCharacter|SwitchTargetRight)))

(event EventBeginPlay
  (if (Pawn|IsLocallyControlled)
    (bind _returnvalue (UserInterface|CreateWidget "/Game/Widget/UX_UI/WB_Hub.WB_Hub_C" 0 self))
    (Variables|Default|SetHubWidget _returnvalue)
    (bind _output_get (Variables|Default|Setref%20Hub _returnvalue))
    (Utilities|FlowControl|Delay 0.2)
    (UserInterface|Viewport|AddtoViewport _output_get 0)
    (EventDispatchers|BindEventtoOnHealthChanged (Variables|Default|GetHealthComponent) (delegate Custom|actualizarHub))
    (EventDispatchers|BindEventtoOnXPChanged (Variables|Default|GetAttribute) (delegate Custom|ActualizarXpBar))
    (bind _asbp_necro_life_player_state (Utilities|Casting|CastToBP_NecroLifePlayerState (Game|GetPlayerState 0)))
    (EventDispatchers|BindEventtoOnShowItem (Variables|/Script/NecroLife.NecroLifePlayerState|GetInventoryComponent _asbp_necro_life_player_state) (delegate Custom|ActualizarInventario))
    (EventDispatchers|AssignOnPosionChange (Variables|/Script/NecroLife.NecroLifePlayerState|GetInventoryComponent _asbp_necro_life_player_state) (delegate Custom|ActualizarPotions))
    (bind _aswb_nombre_player (Utilities|Casting|CastToWB_NombrePlayer (UserInterface|GetUserWidgetObject (Variables|Default|GetWidget))))
    (Default|SetName _aswb_nombre_player (Utilities|String|StringToName (Utilities|GetDisplayName (Game|GetPlayerCharacter 0))))
    (EventDispatchers|BindEventtoOnUpdateObjectiveList (Variables|Default|GetQuestComponent) (delegate Custom|ActualizarListaObjetivos))
    (EventDispatchers|BindEventtoAbilitySlot (Variables|Default|GetAbility) (delegate Custom|abilityCoolDown))
    (CallFunction|SetAbilitySlots)
    (EventDispatchers|BindEventtoGemstoShow (Variables|Default|GetInventory) (delegate Custom|gemsToShow))
    (Variables|Default|SetWeaponMesh (Variables|Default|GetSwordMesh))))

(event EventTick
  (params (DeltaSeconds :type Float%20%28single-precision%29))
  (bind _returnvalue (Transformation|GetActorLocation))
  (bind _ref_hub (Variables|Default|Getref%20Hub))
  (Rendering|Material|SetVectorParameterValue "/Game/Maps/PlayGround/Materials/MPC_OclusionMask.MPC_OclusionMask" "PlayerPosicion" (Utilities|Struct|MakeLinearColor (.x _returnvalue) (.y _returnvalue) (.z _returnvalue) (Variables|/Script/Engine.SpringArmComponent|GetTargetArmLength (Variables|Default|GetCameraBoom))) :!class /Script/Engine.KismetMaterialLibrary)
  (if (Utilities|IsValid _ref_hub)
    (Default|ActualizarMiniMapa _ref_hub (.x _returnvalue) (.y _returnvalue) (Transformation|GetActorRotation))))

(event EventOnInteract
  (params (Interactor :type Actor%20Object%20Reference)))

(fn ConstructionScript)

(fn GetLookatLocation
  (return "0, 0, 0"))

(fn SetAbilitySlots
  (bind _returnvalue (Class|AbilityComponent|GetAbilitySlots (Variables|Default|GetAbility)))
  (Default|SetAbilitiesSlots (Variables|/Game/Widget/UX_UI/WB_Hub.WB_Hub_C|GetWB_AbilityPanel (Variables|Default|Getref%20Hub)) _returnvalue))