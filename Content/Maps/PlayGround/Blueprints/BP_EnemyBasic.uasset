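; Basic enemy character that damages overlapping NecroLifeCharacters and drops loot on death.
; HealthComponent changes update the WB_Enemy life bar and flag damage; at zero health it broadcasts OnMuerte, drops XP, waits briefly, may spawn a random DT_Gemas gem, then destroys itself.
; Attack flags attacking and applies EnemyDamage through Box overlaps.
; It also sets an optional gameplay tag, adjusts walk speed and toggles a target-indicator widget.
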(event Custom|muere?
  (params (NewHealth :type Float%20%28single-precision%29) (MaxHealth :type Float%20%28single-precision%29))
  (bind _returnvalue (Transformation|GetActorTransform))
  (if (<= NewHealth 0.0)
    (bind _aswb_enemy (Utilities|Casting|CastToWB_Enemy (UserInterface|GetWidget (Variables|Default|GetWidget))))
    (Default|UpdateLife _aswb_enemy 0.0)
    (Default|CallOnMuerte)
    (Game|SpawnActorfromClass "/Game/Assets/Items/BP_ItemXP.BP_ItemXP_C" _returnvalue "Undefined" "MultiplyWithRoot" 0 0)
    (Utilities|FlowControl|Delay 1.0)
    (if (< (Math|Random|RandomIntegerinRange 0 100) (Variables|Default|GetSpawnGemRandom))
      (bind _outrownames (DataTable|GetDataTableRowNames "/Game/Assets/DataAssets/DT_Gemas.DT_Gemas"))
      (Game|SpawnActorfromClass "/Game/Assets/Items/BP_ItemGema.BP_ItemGema_C" _returnvalue "Undefined" "MultiplyWithRoot" 0 (Utilities|Struct|MakeDataTableRowHandle "/Game/Assets/DataAssets/DT_Gemas.DT_Gemas" (Utilities|Array|Get(acopy) _outrownames (Math|Random|RandomIntegerinRange 0 (- (Utilities|Array|Length _outrownames) 1)))) 0)
      (Actor|DestroyActor)
      (else
        (Actor|DestroyActor)))
    (else
      (bind _aswb_enemy_2 (Utilities|Casting|CastToWB_Enemy (UserInterface|GetWidget (Variables|Default|GetWidget))))
      (Default|UpdateLife _aswb_enemy_2 (/ NewHealth MaxHealth))
      (Variables|Default|SetbIsEDamaged true))))

(event EventBeginPlay
  (EventDispatchers|BindEventtoOnHealthChanged (Variables|Default|GetHealthComponent) (delegate Custom|muere?))
  (if (GameplayTags|IsGameplayTagValid (Variables|Default|GettagToAsign))
    (Class|NecroLifeEnemyBasic|SetTag (Variables|Default|GettagToAsign))))

(event EventOnTargetStatusChanged
  (params (bIsTarget :type Boolean))
  (bind _targetwidget (Variables|Default|GetTargetWidget))
  (if bIsTarget
    (Rendering|SetVisibility _targetwidget true false)
    (else
      (Rendering|SetVisibility _targetwidget false false))))

(fn ConstructionScript)

(fn UpdateWalkSpeed
  (params (WalkSpeed :type Float%20%28double-precision%29))
  (Variables|/Script/Engine.CharacterMovementComponent|SetMaxWalkSpeed (Variables|Character|GetCharacterMovement) WalkSpeed))

(fn Attack!
  (Variables|Default|SetbIsEAttacking true)
  (CallFunction|DoDamage (Variables|Default|GetEnemyDamage)))

(fn DoDamage
  (params (EnemyDamage :type Float%20%28double-precision%29))
  (for _array_element (Collision|GetOverlappingActors (Variables|Default|GetBox) "/Script/NecroLife.NecroLifeCharacter" :!class /Script/Engine.PrimitiveComponent)
    (bind _asnecro_life_character (Utilities|Casting|CastToNecroLifeCharacter _array_element))
    (Class|UHealthComponent|TakeDamage (Variables|/Script/NecroLife.NecroLifeCharacter|GetHealthComponent _asnecro_life_character) EnemyDamage)))