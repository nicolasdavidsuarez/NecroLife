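; Wave spawner that runs sequential enemy waves and reports each cleared wave to the quest system.
; Waves start after a short delay when the Oleadas quest is added, or when a NecroLifeCharacter enters the trigger box, which then disables its collision.
; Each wave spawns its configured enemy classes and amounts at SpawnPoint.
; A death-event counter advances the waves and updates quest progress through the GameState's QuestComponent.
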(event OnComponentBeginOverlap(Box)
  (params (OverlappedComponent :type Primitive%20Component%20Object%20Reference) (OtherActor :type Actor%20Object%20Reference) (OtherComp :type Primitive%20Component%20Object%20Reference) (OtherBodyIndex :type Integer) (bFromSweep :type Boolean) (SweepResult :type Hit%20Result%20Structure%20%28by%20ref%29))
  (Utilities|Casting|CastToNecroLifeCharacter OtherActor)
  (Collision|SetCollisionEnabled (Variables|Default|GetBox) "NoCollision")
  (CallFunction|StartWave))

(event Custom|ActivateWave
  (params (Quest :type Quest%20Data%20Object%20Reference))
  (if (== Quest "/Game/Maps/PlayGround/Data_Assets/DA_QuestOleadas.DA_QuestOleadas")
    (Utilities|FlowControl|Delay 5.0)
    (CallFunction|StartWave)))

(event EventBeginPlay
  (EventDispatchers|BindEventtoOnQuestAdded (Actor|GetComponentbyClass (Game|GetGameState) "/Script/NecroLife.QuestComponent") (delegate Custom|ActivateWave)))

(event Collision|EventActorBeginOverlap
  (params (OtherActor :type Actor%20Object%20Reference)))

(event EventTick
  (params (DeltaSeconds :type Float%20%28single-precision%29)))

(fn ConstructionScript)

(fn StartWave
  (Variables|Default|SetCurrentWave 0)
  (Variables|Default|SetAliveEnemies 0)
  (CallFunction|SpawnWave))

(fn OnEnemyDied
  (params (Enemy :type Necro%20Life%20Enemy%20Basic%20Object%20Reference))
  (Variables|Default|SetAliveEnemies (- (Variables|Default|GetAliveEnemies) 1))
  (if (== (Variables|Default|GetAliveEnemies) 0)
    (Variables|Default|SetCurrentWave (+ (Variables|Default|GetCurrentWave) 1))
    (if (>= (Variables|Default|GetCurrentWave) (Utilities|Array|Length (Variables|Default|GetWaves)))
      _
      (else
        (CallFunction|SpawnWave)))
    (Class|QuestComponent|UpdateQuestProgress (Actor|GetComponentbyClass (Game|GetGameState) "/Script/NecroLife.QuestComponent") "(TagName=\"Necro_Tags.Oleadas.Oleada\")" 1)))

(fn SpawnWave
  (for _array_element (Utilities|Struct|BreakS_Wave (Utilities|Array|Get(acopy) (Variables|Default|GetWaves) (Variables|Default|GetCurrentWave)))
    (for _index (range 0 (- (.Amount (Utilities|Struct|BreakS_WaveData _array_element)) 1))
      (bind _returnvalue (Game|SpawnActorfromClass (.EnemyClass (Utilities|Struct|BreakS_WaveData _array_element)) (Transformation|GetActorTransform (Variables|Default|GetSpawnPoint)) "AlwaysSpawn" "MultiplyWithRoot" 0 0))
      (EventDispatchers|BindEventtoOnEnemyDied _returnvalue (EventDispatchers|CreateEvent :!event OnEnemyDied))
      (Variables|Default|SetAliveEnemies (+ (Variables|Default|GetAliveEnemies) 1)))))