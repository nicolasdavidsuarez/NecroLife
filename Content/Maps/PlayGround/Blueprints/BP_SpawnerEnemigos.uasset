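; BP_SpawnerEnemigos is an enemy spawner actor that spawns BP_EnemyBasic at its own location, passing along a NavMesh reference.
; On BeginPlay a looping timer fires Spawn every TiempoEntreSpawn, decrementing CantidadEnemigos after each spawn.
; The timer clears only once the count is below zero, so it spawns one more enemy than a non-negative starting count.
; The Spawnear function is an uncalled, unfinished version of the same logic.
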(event Custom|SpawnearEnemigos
  (bind _returnvalue (Utilities|Time|SetTimerbyEvent (delegate Custom|Spawn) (Variables|Components|GettiempoEntreSpawn) true)))

(event Custom|Spawn
  (bind _cantidadenemigos (Variables|Components|GetCantidadEnemigos))
  (if (< _cantidadenemigos 0)
    (Utilities|Time|ClearandInvalidateTimerbyHandle (stale Custom|SpawnearEnemigos _returnvalue))
    (else
      (Game|SpawnActorfromClass "/Game/Maps/PlayGround/Blueprints/BP_EnemyBasic.BP_EnemyBasic_C" (Math|Transform|MakeTransform (Transformation|GetActorLocation) "0, 0, 0" "1.000000,1.000000,1.000000") "AdjustIfPossibleButAlwaysSpawn" "MultiplyWithRoot" 0 (Variables|Components|GetNavMesh) 0)
      (Math|Integer|DecrementInt _cantidadenemigos))))

(event EventBeginPlay
  (CallFunction|SpawnearEnemigos))

(event Collision|EventActorBeginOverlap
  (params (OtherActor :type Actor%20Object%20Reference)))

(event EventTick
  (params (DeltaSeconds :type Float%20%28single-precision%29)))

(fn ConstructionScript)

(fn Spawnear
  (Utilities|Time|SetTimerbyEvent 0 (Variables|Components|GettiempoEntreSpawn)))