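; Melee enemy Blueprint, named for wave-based combat, that exposes functions for movement speed and a close-range attack.
; WalkSpeed sets the CharacterMovement max walk speed, while BeginPlay, Tick and construction only defer to the parent.
; Attack queries BP_Character actors overlapping its Box, casts each to BP_EnemyWaveMelee and applies fixed damage through that actor's HealthComponent.
; The OnEnemyMuerte death handler is an empty stub.
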(event Collision|EventActorBeginOverlap
  (params (OtherActor :type Actor%20Object%20Reference))
  (|CallParentFunction OtherActor) ; This node is disabled and will not be called.\nDrag off pins to build functionality.
)

(event EventTick
  (params (DeltaSeconds :type Float%20%28single-precision%29))
  (|CallParentFunction DeltaSeconds))

(event EventBeginPlay
  (|CallParentFunction))

(fn ConstructionScript
  (|CallParentFunction))

(fn WalkSpeed
  (params (WalkSpeed :type Float%20%28double-precision%29))
  (Variables|/Script/Engine.CharacterMovementComponent|SetMaxWalkSpeed (Variables|Character|GetCharacterMovement) WalkSpeed))

(fn Attack
  (for _array_element (Collision|GetOverlappingActors (Variables|Default|GetBox) "/Game/Maps/PlayGround/Blueprints/BP_Character.BP_Character_C" :!class /Script/Engine.PrimitiveComponent)
    (bind _asbp_enemy_wave_melee (Utilities|Casting|CastToBP_EnemyWaveMelee _array_element))
    (Class|UHealthComponent|TakeDamage (Variables|/Script/NecroLife.NecroLifeEnemyBasic|GetHealthComponent _asbp_enemy_wave_melee) 5.0)))

(fn OnEnemyMuerte)