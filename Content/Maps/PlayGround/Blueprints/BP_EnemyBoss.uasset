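; Corrupted wolf boss enemy that advances a quest and can drop a gem when it dies.
; SetHealthBar pushes the life percent to the WB_Enemy widget on its widget component.
; OnDie sets the death flag and reports the kill to the GameState's QuestComponent under the LoboCorrompido objective tag.
; After a short delay it rolls against PickupSpawnChance to spawn a BP_ItemGema at its transform, using a random DT_Gemas row.
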(event EventOnDie
  (Variables|Default|SetMuerte true)
  (Class|QuestComponent|UpdateQuestProgress (Actor|GetComponentbyClass (Game|GetGameState) "/Script/NecroLife.QuestComponent") "(TagName=\"Necro_Tags.MisionLoboCorrompido.LoboCorrompido\")" 1)
  (Utilities|FlowControl|Delay 1.0)
  (if (< (Math|Random|RandomIntegerinRange 0 100) (Variables|Default|GetPickupSpawnChance))
    (bind _outrownames (DataTable|GetDataTableRowNames "/Game/Assets/DataAssets/DT_Gemas.DT_Gemas"))
    (Game|SpawnActorfromClass "/Game/Assets/Items/BP_ItemGema.BP_ItemGema_C" (Transformation|GetActorTransform) "Undefined" "MultiplyWithRoot" 0 (Utilities|Struct|MakeDataTableRowHandle "/Game/Assets/DataAssets/DT_Gemas.DT_Gemas" (Utilities|Array|Get(acopy) _outrownames (Math|Random|RandomIntegerinRange 0 (- (Utilities|Array|Length _outrownames) 1)))) 0)))

(event EventSetHealthBar
  (params (Percent :type Float%20%28single-precision%29))
  (bind _aswb_enemy (Utilities|Casting|CastToWB_Enemy (UserInterface|GetWidget (Variables|Default|GetWidget))))
  (Default|UpdateLife _aswb_enemy Percent))

(fn ConstructionScript)