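; BP_EnemyLobo is a forest wolf enemy that counts toward the Aullidos mission and drops rewards on death.
; Health changes update its WB_Enemy life widget; at zero it sets Muerte, spawns XP and advances the QuestComponent on the GameState.
; After a short delay, a chance roll either spawns a random DT_Gemas gem or destroys the actor; only the no-drop branch calls DestroyActor.
; Attack and damage events set state flags.
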(event Custom|muere?
  (params (NewHealth :type Float%20%28single-precision%29) (MaxHealth :type Float%20%28single-precision%29))
  (bind _returnvalue (Transformation|GetActorTransform))
  (if (<= NewHealth 0.0)
    (bind _aswb_enemy (Utilities|Casting|CastToWB_Enemy (UserInterface|GetWidget (Variables|Default|GetWidget))))
    (Default|UpdateLife _aswb_enemy 0.0)
    (Game|SpawnActorfromClass "/Game/Assets/Items/BP_ItemXP.BP_ItemXP_C" _returnvalue "Undefined" "MultiplyWithRoot" 0 0)
    (Variables|Default|SetbMuerte true)
    (Class|QuestComponent|UpdateQuestProgress (Actor|GetComponentbyClass (Game|GetGameState) "/Script/NecroLife.QuestComponent") "(TagName=\"Necro_Tags.MisionAullidos.LobosBosque\")" 1)
    (Utilities|FlowControl|Delay 1.0)
    (if (< (Math|Random|RandomIntegerinRange 0 100) (Variables|Default|GetPickupSpawnChance))
      (bind _outrownames (DataTable|GetDataTableRowNames "/Game/Assets/DataAssets/DT_Gemas.DT_Gemas"))
      (Game|SpawnActorfromClass "/Game/Assets/Items/BP_ItemGema.BP_ItemGema_C" _returnvalue "Undefined" "MultiplyWithRoot" 0 (Utilities|Struct|MakeDataTableRowHandle "/Game/Assets/DataAssets/DT_Gemas.DT_Gemas" (Utilities|Array|Get(acopy) _outrownames (Math|Random|RandomIntegerinRange 0 (- (Utilities|Array|Length _outrownames) 1)))) 0)
      (else
        (Actor|DestroyActor)))
    (else
      (bind _aswb_enemy_2 (Utilities|Casting|CastToWB_Enemy (UserInterface|GetWidget (Variables|Default|GetWidget))))
      (Default|UpdateLife _aswb_enemy_2 (/ NewHealth MaxHealth)))))

(event EventBeginPlay
  (EventDispatchers|BindEventtoOnHealthChanged (Variables|Default|GetHealthComponent) (delegate Custom|muere?)))

(event EventOnAttack
  (Variables|Default|SetbIsAttacking false))

(event EventOnTakeDamage
  (Variables|Default|SetbIsEDamaged true))

(fn ConstructionScript)